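; AI controller for guard NPCs that runs the GuardBehavior tree on the PatrolData blackboard.
; Perception updates write sensed actors lacking the "Enemy" tag to the blackboard's enemy key and clear it when sensing fails.
; Each tick, the controlled TP_Character's Aiming and Shooting flags mirror whether a valid focus actor exists.
; BeginPlay also caches the pawn's hero animation instance.
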(event `self.ReceiveBeginPlay`
  (bind _blackboardcomponent (`self.UseBlackboard` "/Game/Dynamic/NPC/AI/PatrolData.PatrolData"))
  (set `self.BlackBoardComp` _blackboardcomponent)
  (`self.RunBehaviorTree` "/Game/Dynamic/NPC/AI/GuardBehavior.GuardBehavior")
  (bind _astp_character (cast `/Game/Dynamic/NPC/Behavior/TP_Character` (`self.K2_GetPawn`)))
  (bind _asue4asp_hero_tpp_anim_blueprint (cast `/Game/Dynamic/NPC/Animations/UE4ASP_HeroTPP_AnimBlueprint` (`SkeletalMeshComponent.GetAnimInstance` (`Character.Mesh` _astp_character))))
  (set `self.AnimInstance` _asue4asp_hero_tpp_anim_blueprint))

(event `self.ReceiveTick`
  (params (DeltaSeconds :type "Float (single-precision)"))
  (bind _returnvalue (`KismetSystemLibrary.IsValid` (`self.GetFocusActor`)))
  (bind _astp_character (cast `/Game/Dynamic/NPC/Behavior/TP_Character` (`self.K2_GetPawn`)))
  (set `/Game/Dynamic/NPC/Behavior/TP_Character.Aiming` _returnvalue _astp_character)
  (set `/Game/Dynamic/NPC/Behavior/TP_Character.Shooting` _returnvalue _astp_character))

(event `self.AIPerception.OnTargetPerceptionUpdated`
  (params (Actor :type "Actor Object Reference") (Stimulus :type "AIStimulus Structure"))
  (`/Engine/EditorBlueprintResources/StandardMacros.IsValid` Actor
    (:`Is Valid`
      (if (`self.ActorHasTag` Actor "Enemy")
        _
        (elif (`.bSuccessfullySensed` (break `AIStimulus` Stimulus))
          (`BlackboardComponent.SetValueAsObject` (`self.BlackBoardComp`) (`self.EnemyKey`) Actor)
          (else
            (`BlackboardComponent.ClearValue` (`self.BlackBoardComp`) (`self.EnemyKey`))))))))

(fn `UserConstructionScript`)