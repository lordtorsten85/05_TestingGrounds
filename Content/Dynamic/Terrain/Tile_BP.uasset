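; Terrain tile actor for an infinite terrain system, with a lockable barrier and an Arrow marking the attach transform.
; The barrier starts solid and red, then turns passable and green while the player is inside LockingVolume.
; When the player leaves that volume, the barrier relocks and InfinateTerrainGameMode is told to spawn a tile.
; The tile destroys itself when the player enters its DestroyTile volume.
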(event `self.ReceiveBeginPlay`
  (`self.Lock`))

(event `self.LockingVolume.OnComponentBeginOverlap`
  (params (OverlappedComponent :type "PrimitiveComponent Object Reference") (OtherActor :type "Actor Object Reference") (OtherComp :type "PrimitiveComponent Object Reference") (OtherBodyIndex :type Integer) (bFromSweep :type Boolean) (SweepResult :type "HitResult Structure (by ref)"))
  (`self.IsPlayerActor` OtherActor
    (:`True`
      (`self.Unlock`))))

(event `self.LockingVolume.OnComponentEndOverlap`
  (params (OverlappedComponent :type "PrimitiveComponent Object Reference") (OtherActor :type "Actor Object Reference") (OtherComp :type "PrimitiveComponent Object Reference") (OtherBodyIndex :type Integer))
  (`self.IsPlayerActor` OtherActor
    (:`True`
      (`self.Lock`)
      (bind _asinfinate_terrain_game_mode (cast `/Game/Dynamic/InfinateTerrainGameMode` (`GameplayStatics.GetGameMode`)))
      (`/Game/Dynamic/InfinateTerrainGameMode.SpawnTile` _asinfinate_terrain_game_mode))))

(event `self.DestroyTile.OnComponentBeginOverlap`
  (params (OverlappedComponent :type "PrimitiveComponent Object Reference") (OtherActor :type "Actor Object Reference") (OtherComp :type "PrimitiveComponent Object Reference") (OtherBodyIndex :type Integer) (bFromSweep :type Boolean) (SweepResult :type "HitResult Structure (by ref)"))
  (`self.IsPlayerActor` OtherActor
    (:`True`
      (`self.K2_DestroyActor`))))

(fn `GetAttachLocation`
  (returns (AttachPoint :type "Transform Structure"))
  (return (`KismetMathLibrary.MakeTransform` (.location (`SceneComponent.K2_GetComponentToWorld` (`self.Arrow`))) (.rotation (`SceneComponent.K2_GetComponentToWorld` (`self.Arrow`))))))

(fn `Lock`
  (`PrimitiveComponent.SetCollisionEnabled` (`self.Barrier`) "QueryAndPhysics")
  (`PrimitiveComponent.SetMaterial` (`self.Barrier`) 0 "/Game/Dynamic/Terrain/RedBarrier.RedBarrier"))

(fn `Unlock`
  (`PrimitiveComponent.SetCollisionEnabled` (`self.Barrier`) "NoCollision")
  (`PrimitiveComponent.SetMaterial` (`self.Barrier`) 0 "/Game/Dynamic/Terrain/GreenBarrier.GreenBarrier"))

(fn `UserConstructionScript`)